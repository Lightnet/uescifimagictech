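; BP_WaterBottle01 is a water bottle pickup prop that adds its item to an inventory when interacted with.
; Hovering shows or hides a lazily created pickup widget, and Tick yaws a text label toward the first player's pawn.
; Interaction removes the widget, casts the passed Pawn to a Controller, appends SItem through the inventory message getter and setter, then destroys the actor.
; Label-text switching logic is present but never runs.
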(event `self.ReceiveTick`
  (params (DeltaSeconds :type "Float (single-precision)"))
  (`parent.ReceiveTick` DeltaSeconds)
  (`self.Update Camera Face Text`))

(event `/Game/scifimagictech/gamemodes/BPIHover.InteractHover`
  (params (bHover :type Boolean))
  ;[1 1 1] Hover
  (if bHover
    (`/Engine/EditorBlueprintResources/StandardMacros.IsValid` (`self.BPW_Pickup`)
      (:`Is Valid`
        _)
      (:`Is Not Valid`
        (bind _returnvalue (`|CreateWidget` "/Game/scifimagictech/ui/BPW_Pickup.BPW_Pickup_C"))
        (bind _output_get (set `self.BPW_Pickup` _returnvalue))))
    (`UserWidget.AddToViewport` _output_get 0)
    (else
      (`Widget.RemoveFromParent` (`self.BPW_Pickup`)))))

(event `/Game/scifimagictech/gamemodes/BPIInteract.ActorInteract`
  (params (bPress :type Boolean) (Pawn :type "Actor Object Reference"))
  ;[1 1 1] Interact
  (`Widget.RemoveFromParent` (`self.BPW_Pickup`))
  (bind _ascontroller (cast `Controller` Pawn))
  (bind _items (message `/Game/scifimagictech/gamemodes/BPIInventory.get Inventory` _ascontroller))
  (`KismetArrayLibrary.Array_Add` _items (`self.SItem`))
  (message `/Game/scifimagictech/gamemodes/BPIInventory.set Inventory` _ascontroller _items)
  (`self.K2_DestroyActor`))

(event `Update Camera Face Text`
  ;[1 1 1] Face Direction Text
  (`SceneComponent.K2_SetRelativeRotation` (`self.TextRender`) (`KismetMathLibrary.MakeRotator` 0.0 0.0 (+ (.yaw (`KismetMathLibrary.FindLookAtRotation` (`self.K2_GetActorLocation` (`GameplayStatics.GetPlayerPawn` 0)) (`self.K2_GetActorLocation`))) 180.0)) false false))

(fn `UserConstructionScript`
  (`parent.UserConstructionScript`))