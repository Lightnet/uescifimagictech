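; BP_Chest is an interactable chest prop that opens a chest UI widget when the player interacts with it.
; Each tick its floating text label turns on yaw only to face the player pawn.
; The hover event adds or removes brackets around the label to show focus.
; On interact it creates the BPW_Chest widget if no valid one is cached, then adds it to the viewport.
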(event `self.ReceiveTick`
  (params (DeltaSeconds :type "Float (single-precision)"))
  ;[1 1 1] Look
  (`SceneComponent.K2_SetRelativeRotation` (`self.TextRender`) (`KismetMathLibrary.MakeRotator` 0.0 0.0 (+ (.yaw (`KismetMathLibrary.FindLookAtRotation` (`self.K2_GetActorLocation` (`GameplayStatics.GetPlayerPawn` 0)) (`self.K2_GetActorLocation`))) 180.0)) false false))

(event `/Game/scifimagictech/gamemodes/BPIHover.InteractHover`
  (params (bHover :type Boolean))
  ;[1 1 1] Hover
  (if bHover
    (set `self.DisplayText` "[Chest]")
    (else
      (set `self.DisplayText` "Chest")))
  (`TextRenderComponent.K2_SetText` (`self.TextRender`) (`self.DisplayText`)))

(event `/Game/scifimagictech/gamemodes/BPIInteract.ActorInteract`
  (params (bPress :type Boolean))
  (`/Engine/EditorBlueprintResources/StandardMacros.IsValid` (`self.BPWChest`)
    (:`Is Valid`
      _)
    (:`Is Not Valid`
      (bind _returnvalue (`|CreateWidget` "/Game/scifimagictech/ui/BPW_Chest.BPW_Chest_C"))
      (bind _output_get (set `self.BPWChest` _returnvalue))))
  (`UserWidget.AddToViewport` _output_get 0))

(fn `UserConstructionScript`
  (`parent.UserConstructionScript`))